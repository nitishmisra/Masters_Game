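; Boss character that fires AI_Projectile at intervals while the player stands in one of its eight shooting areas.
; BeginPlay fills parallel arrays of trigger areas and projectile spawners, paired by index.
; Tick polls the areas for player overlap, stores the matching spawner as ActiveBox and calls StartStooting.
; Its one-second Delay throttles the per-frame calls, then spawns the projectile at the current ActiveBox's location and rotation.
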(event Custom|Start%20Stooting
  (bind _active_box (Variables|Default|GetActive%20Box))
  (bind _returnvalue (Transformation|GetWorldLocation _active_box))
  (bind _returnvalue_2 (Transformation|GetWorldRotation _active_box))
  (bind _returnvalue_3 (Math|Transform|MakeTransform _returnvalue _returnvalue_2))
  (bind (_location _rotation) (Math|Transform|BreakTransform _returnvalue_3))
  (Utilities|FlowControl|Delay 1.0)
  (Game|SpawnActorfromClass "/Game/FirstPersonBP/Blueprints/AI_Projectile.AI_Projectile_C" (Math|Transform|MakeTransform _location _rotation) "Undefined" 0 0))

(event EventBeginPlay
  (Utilities|FlowControl|Sequence
    (:then_0
      (Variables|Default|SetShooting%20Triggerbox%20Array (Utilities|Array|MakeArray (Variables|Default|GetShoot%20Area%201) (Variables|Default|GetShoot%20Area%202) (Variables|Default|GetShoot%20Area%203) (Variables|Default|GetShoot%20Area%204) (Variables|Default|GetShoot%20Area%205) (Variables|Default|GetShoot%20Area%206) (Variables|Default|GetShoot%20Area%207) (Variables|Default|GetShoot%20Area%208))))
    (:then_1
      (Variables|Default|SetPrijectile%20Spawnner%20Array (Utilities|Array|MakeArray (Variables|Default|GetProjectile%20Spawner1) (Variables|Default|GetProjectile%20Spawner2) (Variables|Default|GetProjectile%20Spawner3) (Variables|Default|GetProjectile%20Spawner4) (Variables|Default|GetProjectile%20Spawner5) (Variables|Default|GetProjectile%20Spawner6) (Variables|Default|GetProjectile%20Spawner7) (Variables|Default|GetProjectile%20Spawner8))))))

(event Collision|EventActorBeginOverlap
  (params (OtherActor :type Actor%20Object%20Reference)))

(event EventTick
  (params (DeltaSeconds :type Float%20%28single-precision%29))
  (Utilities|FlowControl|Sequence
    (:then_0
      (for (_array_element _array_index) (Variables|Default|GetShooting%20Triggerbox%20Array)
        (if (Collision|IsOverlappingActor _array_element (Game|Player|GetPlayerPawn 0) :!class /Script/Engine.PrimitiveComponent)
          (Utilities|FlowControl|Sequence
            (:then_0
              (Variables|Default|SetActive%20Box (Utilities|Array|Get(acopy) (Variables|Default|GetPrijectile%20Spawnner%20Array) _array_index)))
            (:then_1
              (CallFunction|StartStooting)))
          (elif (Collision|IsOverlappingActor _array_element (Game|Player|GetPlayerPawn 0) :!class /Script/Engine.PrimitiveComponent)
            (Utilities|FlowControl|Sequence
              (:then_0
                (Variables|Default|SetActive%20Box (Utilities|Array|Get(acopy) (Variables|Default|GetPrijectile%20Spawnner%20Array) _array_index)))
              (:then_1
                (CallFunction|StartStooting)))))))
    (:then_1
      (Utilities|FlowControl|Gate true))))

(fn ConstructionScript)